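; NPC AI controller that runs a guard behavior tree and tracks perceived targets for it.
; On BeginPlay it initializes the PatrolData blackboard, starts GuardBehaviour and caches the blackboard component.
; AI Perception updates pass through a helper that ignores actors tagged Enemy, storing any other sensed actor in the EnemyKey blackboard value and clearing that key when sensing fails.
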(event OnTargetPerceptionUpdated(AIPerception)
  (params (Actor :type Actor%20Object%20Reference) (Stimulus :type AI%20Stimulus%20Structure))
  (CallFunction|UpdateBlackboardEnemyKey Stimulus Actor Actor))

(event EventBeginPlay
  (bind _blackboardcomponent (Class|AIController|UseBlackboard "/Game/Dynamic/Character/AI/PatrolData.PatrolData"))
  (AI|RunBehaviorTree "/Game/Dynamic/Character/AI/GuardBehaviour.GuardBehaviour")
  (Variables|Default|SetBlackboardComp _blackboardcomponent))

(fn ConstructionScript)

(fn UpdateBlackboardEnemyKey
  (params (AIStimulus :type AI%20Stimulus%20Structure%20%28by%20ref%29) (ObjectValue :type Object%20Object%20Reference) (self2 :type Actor%20Object%20Reference))
  (bind _blackboardcomp (Variables|Default|GetBlackboardComp))
  (bind _enemykey (Variables|Default|GetEnemyKey))
  (if (not (Actor|ActorHasTag self2 "Enemy"))
    (if (.bSuccessfullySensed (Utilities|Struct|BreakAIStimulus AIStimulus))
      (AI|Components|Blackboard|SetValueasObject _blackboardcomp _enemykey ObjectValue)
      (else
        (AI|Components|Blackboard|ClearValue _blackboardcomp _enemykey)))))