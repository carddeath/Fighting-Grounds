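; Behavior tree task that makes an AI-controlled Character aim and shoot at a target.
; On execute it sets the aiming and shooting flags on the pawn and focuses the controller on the actor in the Target blackboard key.
; It never finishes execution itself, so it stays active until aborted.
; On abort it clears both flags and the focus, then finishes the abort.
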(event EventReceiveExecuteAI
  (params (OwnerController :type AI%20Controller%20Object%20Reference) (ControlledPawn :type Pawn%20Object%20Reference))
  (bind _ascharacter (Utilities|Casting|CastToCharacter ControlledPawn))
  (Variables|/Game/Dynamic/Character/Behaviour/Character.Character_C|SetAimingChar _ascharacter true)
  (Variables|/Game/Dynamic/Character/Behaviour/Character.Character_C|SetShootingChar _ascharacter true)
  (AI|SetFocus OwnerController (AI|BehaviorTree|GetBlackboardValueasActor (Variables|Default|GetTarget))))

(event EventReceiveAbortAI
  (params (OwnerController :type AI%20Controller%20Object%20Reference) (ControlledPawn :type Pawn%20Object%20Reference))
  (bind _ascharacter (Utilities|Casting|CastToCharacter ControlledPawn))
  (Variables|/Game/Dynamic/Character/Behaviour/Character.Character_C|SetAimingChar _ascharacter false)
  (Variables|/Game/Dynamic/Character/Behaviour/Character.Character_C|SetShootingChar _ascharacter false)
  (AI|ClearFocus OwnerController)
  (Class|BTTaskBlueprintBase|FinishAbort))